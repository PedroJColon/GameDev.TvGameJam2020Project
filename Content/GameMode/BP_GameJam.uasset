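; Game mode for a game jam title that runs a per-level countdown, the HUD, music and end-of-level screens.
; BeginPlay sets the time limit from the level selected in BP_GameInstance and starts a looping DecrementTimer.
; When time reaches zero, input is disabled and GameOver runs.
; GameOver and six duplicated per-level LevelComplete events pause the timer, switch to UI input, show their widget and fade out music.
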(event Custom|GameOver
  (bind _returnvalue (Game|GetPlayerController 0))
  ;[1 1 1] Game Over Script
  (Utilities|Time|PauseTimerbyHandle (Variables|Default|GetTimer))
  (Input|SetInputModeUIOnly _returnvalue 0 "DoNotLock")
  (Variables|/Script/Engine.PlayerController|SetbShowMouseCursor _returnvalue true)
  (bind _returnvalue_2 (UserInterface|CreateWidget "/Game/UI/WBP_GameOver.WBP_GameOver_C"))
  (UserInterface|Viewport|AddtoViewport _returnvalue_2 0)
  (Audio|Components|Audio|FadeOut (Variables|Default|GetGameMusic) 1.0 0.0 "Linear" :!class /Script/Engine.AudioComponent))

(event Custom|Level%20Complete%202
  (bind _returnvalue (Game|GetPlayerController 0))
  ;[1 1 1] Level Completed For Level 2
  (Utilities|Time|PauseTimerbyHandle (Variables|Default|GetTimer))
  (Input|DisableInput (Game|GetPlayerCharacter 0) _returnvalue)
  (Input|SetInputModeUIOnly _returnvalue 0 "DoNotLock")
  (Variables|/Script/Engine.PlayerController|SetbShowMouseCursor _returnvalue true)
  (bind _returnvalue_2 (UserInterface|CreateWidget "/Game/UI/LevelCompleteUI/WBP_LevelComplete2.WBP_LevelComplete2_C"))
  (UserInterface|Viewport|AddtoViewport _returnvalue_2 0)
  (Audio|Components|Audio|FadeOut (Variables|Default|GetGameMusic) 1.0 0.0 "Linear" :!class /Script/Engine.AudioComponent))

(event Custom|Level%20Complete%203
  (bind _returnvalue (Game|GetPlayerController 0))
  ;[1 1 1] Level Completed For Level 3
  (Utilities|Time|PauseTimerbyHandle (Variables|Default|GetTimer))
  (Input|DisableInput (Game|GetPlayerCharacter 0) _returnvalue)
  (Input|SetInputModeUIOnly _returnvalue 0 "DoNotLock")
  (Variables|/Script/Engine.PlayerController|SetbShowMouseCursor _returnvalue true)
  (bind _returnvalue_2 (UserInterface|CreateWidget "/Game/UI/LevelCompleteUI/WBP_LevelComplete3.WBP_LevelComplete3_C"))
  (UserInterface|Viewport|AddtoViewport _returnvalue_2 0)
  (Audio|Components|Audio|FadeOut (Variables|Default|GetGameMusic) 1.0 0.0 "Linear" :!class /Script/Engine.AudioComponent))

(event Custom|Level%20Complete%204
  (bind _returnvalue (Game|GetPlayerController 0))
  ;[1 1 1] Level Completed For Level 4
  (Utilities|Time|PauseTimerbyHandle (Variables|Default|GetTimer))
  (Input|DisableInput (Game|GetPlayerCharacter 0) _returnvalue)
  (Input|SetInputModeUIOnly _returnvalue 0 "DoNotLock")
  (Variables|/Script/Engine.PlayerController|SetbShowMouseCursor _returnvalue true)
  (bind _returnvalue_2 (UserInterface|CreateWidget "/Game/UI/LevelCompleteUI/WBP_LevelComplete4.WBP_LevelComplete4_C"))
  (UserInterface|Viewport|AddtoViewport _returnvalue_2 0)
  (Audio|Components|Audio|FadeOut (Variables|Default|GetGameMusic) 1.0 0.0 "Linear" :!class /Script/Engine.AudioComponent))

(event Custom|Level%20Complete%205
  (bind _returnvalue (Game|GetPlayerController 0))
  ;[1 1 1] Level Completed For Level 5
  (Utilities|Time|PauseTimerbyHandle (Variables|Default|GetTimer))
  (Input|DisableInput (Game|GetPlayerCharacter 0) _returnvalue)
  (Input|SetInputModeUIOnly _returnvalue 0 "DoNotLock")
  (Variables|/Script/Engine.PlayerController|SetbShowMouseCursor _returnvalue true)
  (bind _returnvalue_2 (UserInterface|CreateWidget "/Game/UI/LevelCompleteUI/WBP_LevelComplete5.WBP_LevelComplete5_C"))
  (UserInterface|Viewport|AddtoViewport _returnvalue_2 0)
  (Audio|Components|Audio|FadeOut (Variables|Default|GetGameMusic) 1.0 0.0 "Linear" :!class /Script/Engine.AudioComponent))

(event Custom|Level%20Complete%206
  (bind _returnvalue (Game|GetPlayerController 0))
  ;[1 1 1] Level Completed For Level 6
  (Utilities|Time|PauseTimerbyHandle (Variables|Default|GetTimer))
  (Input|DisableInput (Game|GetPlayerCharacter 0) _returnvalue)
  (Input|SetInputModeUIOnly _returnvalue 0 "DoNotLock")
  (Variables|/Script/Engine.PlayerController|SetbShowMouseCursor _returnvalue true)
  (bind _returnvalue_2 (UserInterface|CreateWidget "/Game/UI/LevelCompleteUI/WBP_LevelComplete6.WBP_LevelComplete6_C"))
  (UserInterface|Viewport|AddtoViewport _returnvalue_2 0)
  (Audio|Components|Audio|FadeOut (Variables|Default|GetGameMusic) 1.0 0.0 "Linear" :!class /Script/Engine.AudioComponent))

(event Custom|Level%20Complete
  (bind _returnvalue (Game|GetPlayerController 0))
  ;[1 1 1] Level Completed For Level 1
  (Utilities|Time|PauseTimerbyHandle (Variables|Default|GetTimer))
  (Input|DisableInput (Game|GetPlayerCharacter 0) _returnvalue)
  (Input|SetInputModeUIOnly _returnvalue 0 "DoNotLock")
  (Variables|/Script/Engine.PlayerController|SetbShowMouseCursor _returnvalue true)
  (bind _returnvalue_2 (UserInterface|CreateWidget "/Game/UI/LevelCompleteUI/WBP_LevelComplete.WBP_LevelComplete_C"))
  (UserInterface|Viewport|AddtoViewport _returnvalue_2 0)
  (Audio|Components|Audio|FadeOut (Variables|Default|GetGameMusic) 1.0 0.0 "Linear" :!class /Script/Engine.AudioComponent))

(event EventBeginPlay
  (Utilities|FlowControl|Sequence
    (:then_0
      ;[1 1 1] Show HUD
      (bind _returnvalue (UserInterface|CreateWidget "/Game/UI/HUD/WBP_HUD.WBP_HUD_C"))
      (UserInterface|Viewport|AddtoViewport _returnvalue 0))
    (:then_1
      ;[1 1 1] Play Game Music
      (Audio|Components|Audio|Play (Variables|Default|GetGameMusic) 0.0))
    (:then_2
      ;[1 1 1] Set Game Time Limit Based On Level Selected
      (bind _asbp_game_instance (Utilities|Casting|CastToBP_GameInstance (Game|GetGameInstance)))
      (Variables|Default|SetGameTimer (Utilities|Select :Index (Variables|/Game/FrameWork/BP_GameInstance.BP_GameInstance_C|GetE_LevelSelected _asbp_game_instance) :NewEnumerator0 (Variables|Default|GetLevel1_Timer) :NewEnumerator1 (Variables|Default|GetLevel2_Timer) :NewEnumerator2 (Variables|Default|GetLevel3_Timer) :NewEnumerator3 (Variables|Default|GetLevel4_Timer) :NewEnumerator4 (Variables|Default|GetLevel5_Timer) :NewEnumerator5 (Variables|Default|GetLevel6_Timer))))
    (:then_3
      ;[1 1 1] Decrement Timer
      (bind _returnvalue_2 (Utilities|Time|SetTimerbyFunctionName 0 "DecrementTimer" (Variables|Default|GetDecreaseTime) true))
      (Variables|Default|SetTimer _returnvalue_2))))

(fn ConstructionScript)

(fn DecrementTimer
  (bind _returnvalue (Game|GetPlayerController 0))
  (bind _output_get (Variables|Default|SetGameTimer (- (Variables|Default|GetGameTimer) 1)))
  (if (== _output_get 0)
    (bind _asbp_player_controller (Utilities|Casting|CastToBP_PlayerController _returnvalue))
    (Input|DisableInput _asbp_player_controller _returnvalue)
    (CallFunction|GameOver)))